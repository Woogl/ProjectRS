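; Player controller that handles level loading, quitting and mouse-wheel camera zoom through the Gameplay Cameras variable table.
; P opens the battle arena level and Escape quits the game.
; The mouse wheel steps the X of a vector camera variable within a clamped range, presumably the boom offset.
; On Possess and BeginPlay, another vector camera variable takes the pawn's BaseEyeHeight as its Z to set the camera height.
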(event `Key|P`
  (params (Key :type "Key Structure"))
  (:`Pressed`
    (`GameplayStatics.OpenLevelBySoftObjectPtr` "/Game/Maps/LV_BattleArena.LV_BattleArena")))

(event `Key|Escape`
  (params (Key :type "Key Structure"))
  (:`Pressed`
    (`KismetSystemLibrary.QuitGame` null "Quit")))

(event `Key|MouseScrollUp`
  (params (Key :type "Key Structure"))
  (bind _returnvalue (`GameplayCameraComponent.GetInitialVariableTable` (`self.GameplayCameraComponent`)))
  (:`Pressed`
    (bind _returnvalue_2 (`BlueprintCameraVariableTableFunctionLibrary.GetVector3CameraVariable` _returnvalue "/Game/Camera/CVC_PlayerCamera.CVC_PlayerCamera.Vector3dCameraVariable_0"))
    (`BlueprintCameraVariableTableFunctionLibrary.SetVector3CameraVariable` _returnvalue "/Game/Camera/CVC_PlayerCamera.CVC_PlayerCamera.Vector3dCameraVariable_0" (`KismetMathLibrary.MakeVector` (`KismetMathLibrary.FClamp` (+ (.x _returnvalue_2) 20.0) -350.0 -100.0) (.y _returnvalue_2) (.z _returnvalue_2)))))

(event `Key|MouseScrollDown`
  (params (Key :type "Key Structure"))
  (bind _returnvalue (`GameplayCameraComponent.GetInitialVariableTable` (`self.GameplayCameraComponent`)))
  (:`Pressed`
    (bind _returnvalue_2 (`BlueprintCameraVariableTableFunctionLibrary.GetVector3CameraVariable` _returnvalue "/Game/Camera/CVC_PlayerCamera.CVC_PlayerCamera.Vector3dCameraVariable_0"))
    (`BlueprintCameraVariableTableFunctionLibrary.SetVector3CameraVariable` _returnvalue "/Game/Camera/CVC_PlayerCamera.CVC_PlayerCamera.Vector3dCameraVariable_0" (`KismetMathLibrary.MakeVector` (`KismetMathLibrary.FClamp` (- (.x _returnvalue_2) 20.0) -350.0 -100.0) (.y _returnvalue_2) (.z _returnvalue_2)))))

(event `self.ReceivePossess`
  (params (PossessedPawn :type "Pawn Object Reference"))
  (`BlueprintCameraVariableTableFunctionLibrary.SetVector3CameraVariable` (`GameplayCameraComponent.GetInitialVariableTable` (`self.GameplayCameraComponent`)) "/Game/Camera/CVC_PlayerCamera.CVC_PlayerCamera.Vector3dCameraVariable_3" (`KismetMathLibrary.MakeVector` 0.0 0.0 (`Pawn.BaseEyeHeight` PossessedPawn))))

(event `self.ReceiveBeginPlay`
  (`BlueprintCameraVariableTableFunctionLibrary.SetVector3CameraVariable` (`GameplayCameraComponent.GetInitialVariableTable` (`self.GameplayCameraComponent`)) "/Game/Camera/CVC_PlayerCamera.CVC_PlayerCamera.Vector3dCameraVariable_3" (`KismetMathLibrary.MakeVector` 0.0 0.0 (`Pawn.BaseEyeHeight` (`self.K2_GetPawn`)))))

(fn `UserConstructionScript`)