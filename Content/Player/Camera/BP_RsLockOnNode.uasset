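; Camera node that keeps the player's locked-on target in view by rotating the camera toward it.
; Each tick it reads the target from the player controller's RsLockOnComponent and, when that target leaves the screen's central zone, interpolates the camera pose rotation to look at it.
; IsInScreenCenter projects the target to screen space and tests it against margins set by HorizontalSlice and VerticalSlice, creating a dead zone without camera correction.
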(event `self.TickCameraNode`
  (params (DeltaTime :type "Float (single-precision)"))
  (bind _camerapose (`self.CameraPose`))
  (bind _returnvalue (`RsLockOnComponent.GetLockedOnTarget` (`Actor.GetComponentByClass` (`self.FindEvaluationContextOwnerActor` "/Script/Rs.RsPlayerController") "/Script/Rs.RsLockOnComponent")))
  (bind _returnvalue_2 (`Actor.K2_GetActorLocation` _returnvalue))
  (`/Engine/EditorBlueprintResources/StandardMacros.IsValid` _returnvalue
    (:`Is Valid`
      (if (not (`self.Is In Screen Center` _returnvalue_2 (`self.Horizontal Slice`) (`self.Vertical Slice`)))
        (bind _returnvalue_3 (`BlueprintCameraPoseFunctionLibrary.SetRotation` (`self.CameraPose`) (`KismetMathLibrary.RInterpTo` (`BlueprintCameraPoseFunctionLibrary.GetRotation` _camerapose) (`KismetMathLibrary.FindLookAtRotation` (`BlueprintCameraPoseFunctionLibrary.GetLocation` _camerapose) _returnvalue_2) DeltaTime (`self.Interp Speed`))))
        (set `self.CameraPose` _returnvalue_3)))))

(fn `Is In Screen Center`
  (params (WorldPosition :type "Vector Structure (by ref)") (HorizontalSlice :type Integer) (VerticalSlice :type Integer))
  (returns (ReturnValue :type Boolean))
  (bind _returnvalue (`self.FindEvaluationContextOwnerActor` "/Script/Rs.RsPlayerController"))
  (bind (_screenposition _returnvalue_2) (`GameplayStatics.ProjectWorldToScreen` _returnvalue WorldPosition))
  (bind (_sizex _sizey) (`PlayerController.GetViewportSize` _returnvalue))
  (bind (_x _y) (`KismetMathLibrary.BreakVector2D` _screenposition))
  (bind _returnvalue_3 (/ _sizey VerticalSlice))
  (bind _returnvalue_4 (/ _sizex HorizontalSlice))
  (if _returnvalue_2
    (return (and (< _x (- _sizex _returnvalue_4)) (> _x _returnvalue_4) (< _y (- _sizey _returnvalue_3)) (> _y _returnvalue_3)))
    (else
      (return false))))