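; Boss02 monster Blueprint that adds a nameplate to the boss and handles its cleanup on death.
; On BeginPlay it creates a character view model for itself and passes it to a WBP_Nameplate widget shown through its NameplateComponent.
; When HealthComponent reports health at or below zero, it destroys the nameplate component and sets a short lifespan so the actor removes itself.
; A node attaching the weapon to the right-hand socket is present but unconnected.
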(event `self.ReceiveBeginPlay`
  (bind _returnvalue (`RsCharacterViewModel.CreateRsCharacterViewModel` self))
  (bind _returnvalue_2 (`|CreateWidget` "/Game/UI/Widgets/WBP_Nameplate.WBP_Nameplate_C" null _returnvalue))
  (`WidgetComponent.SetWidget` (`self.NameplateComponent`) _returnvalue_2))

(event `self.HealthComponent.OnHealthChange`
  (params (NewValue :type "Float (single-precision)"))
  (if (<= NewValue 0.0)
    (`ActorComponent.K2_DestroyComponent` (`self.NameplateComponent`))
    (`self.SetLifeSpan` 10.0)))

(fn `UserConstructionScript`)