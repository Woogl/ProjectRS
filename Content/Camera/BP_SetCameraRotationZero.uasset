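; Blueprint camera node that rewrites the camera pose rotation each tick, keeping pitch and yaw and leaving roll at its zero default.
; A separate NewFunction reads a vector camera variable from the player controller's GameplayCameraComponent initial variable table.
; It returns a point 200 units from the controlled pawn, directly away from that vector's position.
; The tick event does not call this function.
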(event `self.TickCameraNode`
  (params (DeltaTime :type "Float (single-precision)"))
  (bind _camerapose (`self.CameraPose`))
  (bind (_returnvalue_roll _returnvalue_pitch _returnvalue_yaw) (`KismetMathLibrary.BreakRotator` (`BlueprintCameraPoseFunctionLibrary.GetRotation` _camerapose)))
  (bind _returnvalue (`BlueprintCameraPoseFunctionLibrary.SetRotation` _camerapose (`KismetMathLibrary.MakeRotator` 0.0 _returnvalue_pitch _returnvalue_yaw)))
  (set `self.CameraPose` _returnvalue))

(fn `NewFunction`
  (returns (ReturnValue :type "Vector Structure"))
  (bind _returnvalue (`self.FindEvaluationContextOwnerActor` "/Script/Rs.RsPlayerController"))
  (bind _returnvalue_2 (`Actor.K2_GetActorLocation` (`Controller.K2_GetPawn` _returnvalue)))
  (bind _returnvalue_3 (`BlueprintCameraVariableTableFunctionLibrary.GetVector3CameraVariable` (`GameplayCameraComponent.GetInitialVariableTable` (`RsPlayerController.GameplayCameraComponent` _returnvalue)) "/Game/Camera/CVC_PlayerCamera.CVC_PlayerCamera.Vector3dCameraVariable_1"))
  (return (+ _returnvalue_2 (* (`KismetMathLibrary.Normal` (- _returnvalue_3 _returnvalue_2)) -200.0))))