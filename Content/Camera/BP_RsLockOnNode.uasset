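; A Gameplay Camera node Blueprint that turns the camera toward the player's locked-on target.
; Each tick it reads the target from the RsLockOnComponent on the RsPlayerController that owns the evaluation context.
; When the target is valid, it smoothly interpolates the camera pose rotation toward a look-at rotation at the target's location, leaving position untouched.
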(event `self.TickCameraNode`
  (params (DeltaTime :type "Float (single-precision)"))
  (bind _camerapose (`self.CameraPose`))
  (bind _returnvalue (`RsLockOnComponent.GetLockedOnTarget` (`Actor.GetComponentByClass` (`self.FindEvaluationContextOwnerActor` "/Script/Rs.RsPlayerController") "/Script/Rs.RsLockOnComponent")))
  (`/Engine/EditorBlueprintResources/StandardMacros.IsValid` _returnvalue
    (:`Is Valid`
      (bind _returnvalue_2 (`BlueprintCameraPoseFunctionLibrary.SetRotation` (`self.CameraPose`) (`KismetMathLibrary.RInterpTo` (`BlueprintCameraPoseFunctionLibrary.GetRotation` _camerapose) (`KismetMathLibrary.FindLookAtRotation` (`BlueprintCameraPoseFunctionLibrary.GetLocation` _camerapose) (`Actor.K2_GetActorLocation` _returnvalue)) DeltaTime 4.0)))
      (set `self.CameraPose` _returnvalue_2))))