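; BP_RsLockOnNode is a Blueprint camera node that turns the camera toward the player's locked-on target.
; Each tick it finds the owning RsPlayerController, its controlled pawn and the target held by its targeting component.
; When both are valid, it overwrites only the camera pose rotation, using a look-at from pawn location to target location rather than from the camera, with no smoothing.
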(event `self.TickCameraNode`
  (params (DeltaTime :type "Float (single-precision)"))
  (bind _returnvalue (`self.FindEvaluationContextOwnerActor` "/Script/Rs.RsPlayerController"))
  (bind _returnvalue_2 (`Controller.K2_GetPawn` _returnvalue))
  (bind _returnvalue_3 (`RsTargetingComponent.GetLockedOnTarget` (`RsTargetingComponent.GetTargetingComponent` _returnvalue)))
  (`/Engine/EditorBlueprintResources/StandardMacros.IsValid` _returnvalue_2
    (:`Is Valid`
      (`/Engine/EditorBlueprintResources/StandardMacros.IsValid` _returnvalue_3
        (:`Is Valid`
          (bind _returnvalue_4 (`BlueprintCameraPoseFunctionLibrary.SetRotation` (`self.CameraPose`) (`KismetMathLibrary.FindLookAtRotation` (`Actor.K2_GetActorLocation` _returnvalue_2) (`Actor.K2_GetActorLocation` _returnvalue_3))))
          (set `self.CameraPose` _returnvalue_4))))))