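; Demo trigger actor for ProHUD V2 that starts a sample mission when the third-person character enters its box.
; Through the HUD manager it creates the mission from six task objects, some optional, and activates the first task.
; It then enables that task object and adds a pinging world marker on it.
; A DoOnce blocks repeat starts until the mission area's leave event resets it.
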(event `self.Box.OnComponentBeginOverlap`
  (params (OverlappedComponent :type "PrimitiveComponent Object Reference") (OtherActor :type "Actor Object Reference") (OtherComp :type "PrimitiveComponent Object Reference") (OtherBodyIndex :type Integer) (bFromSweep :type Boolean) (SweepResult :type "HitResult Structure (by ref)"))
  (cast `/Game/FabAsset/ProHUDV2/DemoContent/DemoCharacter/ThirdPersonCharacter` OtherActor)
  (`/Engine/EditorBlueprintResources/StandardMacros.DoOnce` false :!label _label
    (:`Completed`
      (`/Game/FabAsset/ProHUDV2/Blueprints/Libraries/BPi_HUDManagerV2.CreateMission` (`/Game/FabAsset/ProHUDV2/Blueprints/Libraries/BP_PHV2_Functions.GetHUDManager`) (`/Game/FabAsset/ProHUDV2/DemoContent/Blueprints/BP_Demo_Functions.GetDemoMissionName`) (make `/Game/FabAsset/ProHUDV2/Blueprints/Structs/S_TextInfo` false (struct :`OutlineSettings` (struct :`OutlineColor` (struct :`A` 1.0)) :`Size` 24.0 :`MonospacedWidth` 1.0) 1.2) (`|MakeArray` (make `/Game/FabAsset/ProHUDV2/Blueprints/Structs/S_Task` (`/Game/FabAsset/ProHUDV2/DemoContent/Blueprints/DemoActor/Mission/BP_DemoTaskObject1.MaterialBillboard` (`/Game/FabAsset/ProHUDV2/DemoContent/Blueprints/BP_Demo_Functions.GetTaskObject1`)) "Task Object 1" "Move to Task 1 and collect your next tasks") (make `/Game/FabAsset/ProHUDV2/Blueprints/Structs/S_Task` (`/Game/FabAsset/ProHUDV2/DemoContent/Blueprints/DemoActor/Mission/BP_DemoTaskObject2.MaterialBillboard` (`/Game/FabAsset/ProHUDV2/DemoContent/Blueprints/BP_Demo_Functions.GetTaskObject2`)) "Task Object 2" "Move to your optional Task 2. You can press Q to switch between active tasks" (struct :`FontInfo` (struct :`OutlineSettings` (struct :`OutlineColor` (struct :`A` 1.0)) :`Size` 24.0 :`MonospacedWidth` 1.0) :`Scale` 1.0 :`ColorAndOpacity` (struct)) true) (make `/Game/FabAsset/ProHUDV2/Blueprints/Structs/S_Task` (`/Game/FabAsset/ProHUDV2/DemoContent/Blueprints/DemoActor/Mission/BP_DemoTaskObject3.MaterialBillboard` (`/Game/FabAsset/ProHUDV2/DemoContent/Blueprints/BP_Demo_Functions.GetTaskObject3`)) "Task Object 3" "Move to Task 3 and collect your next tasks") (make `/Game/FabAsset/ProHUDV2/Blueprints/Structs/S_Task` (`/Game/FabAsset/ProHUDV2/DemoContent/Blueprints/DemoActor/Mission/BP_DemoTaskObject4.MaterialBillboard` (`/Game/FabAsset/ProHUDV2/DemoContent/Blueprints/BP_Demo_Functions.GetTaskObject4`)) "Task Object 4" "Get your optional Task number 4. Press Q to switch between Tasks." (struct :`FontInfo` (struct :`OutlineSettings` (struct :`OutlineColor` (struct :`A` 1.0)) :`Size` 24.0 :`MonospacedWidth` 1.0) :`Scale` 1.0 :`ColorAndOpacity` (struct)) true) (make `/Game/FabAsset/ProHUDV2/Blueprints/Structs/S_Task` (`/Game/FabAsset/ProHUDV2/DemoContent/Blueprints/DemoActor/Mission/BP_DemoTaskObject5.MaterialBillboard` (`/Game/FabAsset/ProHUDV2/DemoContent/Blueprints/BP_Demo_Functions.GetTaskObject5`)) "Task Object 5" "Move to Task number 5" (struct :`FontInfo` (struct :`OutlineSettings` (struct :`OutlineColor` (struct :`A` 1.0)) :`Size` 24.0 :`MonospacedWidth` 1.0) :`Scale` 1.0 :`ColorAndOpacity` (struct)) true) (make `/Game/FabAsset/ProHUDV2/Blueprints/Structs/S_Task` (`/Game/FabAsset/ProHUDV2/DemoContent/Blueprints/DemoActor/Mission/BP_DemoTaskObject6.MaterialBillboard` (`/Game/FabAsset/ProHUDV2/DemoContent/Blueprints/BP_Demo_Functions.GetTaskObject6`)) "Task Object 6" "Move to your last task to FINISH the demo mission.")))
      (bind (_currenttaskobject _currenttaskinfo) (`/Game/FabAsset/ProHUDV2/Blueprints/Libraries/BPi_HUDManagerV2.SetActiveTasks` (`/Game/FabAsset/ProHUDV2/Blueprints/Libraries/BP_PHV2_Functions.GetHUDManager`) (`/Game/FabAsset/ProHUDV2/DemoContent/Blueprints/BP_Demo_Functions.GetDemoMissionName`) (`|MakeSet` 0)))
      (set `/Game/FabAsset/ProHUDV2/DemoContent/Blueprints/DemoActor/Mission/BP_DemoTaskObject1.bUseTask` true (`/Game/FabAsset/ProHUDV2/DemoContent/Blueprints/BP_Demo_Functions.GetTaskObject1`))
      (`/Game/FabAsset/ProHUDV2/Blueprints/Libraries/BPi_HUDManagerV2.AddOrUpdateWorldMarker` (`/Game/FabAsset/ProHUDV2/Blueprints/Libraries/BP_PHV2_Functions.GetHUDManager`) _currenttaskobject (make `/Game/FabAsset/ProHUDV2/Blueprints/Structs/S_WorldMarkerInfo` "/Game/FabAsset/ProHUDV2/Textures/MissionNoti/T_MissionIcon_Active.T_MissionIcon_Active" 1.0 (struct :`R` 1.0 :`G` 0.434589 :`A` 1.0) false (`.ObjectName_23_8198AFFE4B09F234492F5DBDEC0E84C4` (break `/Game/FabAsset/ProHUDV2/Blueprints/Structs/S_Task` _currenttaskinfo)) (struct :`FontInfo` (struct :`OutlineSettings` (struct :`OutlineColor` (struct :`A` 1.0)) :`Size` 24.0 :`MonospacedWidth` 1.0) :`Scale` 1.0 :`ColorAndOpacity` (struct)) false false (struct :`DistanceUnit` "NewEnumerator1" :`DistanceStepskm` 10 :`DistanceStepsm` 1 :`DistanceStepsmi` 10 :`DistanceStepsya` 1) (struct :`FontInfo` (struct :`OutlineSettings` (struct :`OutlineColor` (struct :`A` 1.0)) :`Size` 24.0 :`MonospacedWidth` 1.0) :`Scale` 1.0 :`ColorAndOpacity` (struct)) 0 false true false)))))

(event `self.ReceiveBeginPlay`
  (add `/Game/FabAsset/ProHUDV2/DemoContent/Blueprints/DemoActor/Mission/BP_MissionArea.OnLeaveMissionArea` (`/Game/FabAsset/ProHUDV2/DemoContent/Blueprints/BP_Demo_Functions.GetMissionArea`) (delegate `OnLeaveMissionArea_Event_0`)))

(event `OnLeaveMissionArea_Event_0`
  (goto _label :!via `Reset`))

(fn `UserConstructionScript`)