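; BP_MinimapZoomIn is a ProHUDV2 demo trigger that zooms the minimap in or out, depending on its ZoomIn flag.
; When the ThirdPersonCharacter enters the box, it waits briefly, steps the clamped ZoomValue on the first BP_MinimapArea found, then updates the HUD manager.
; A point light, colored green or red by the construction script, double-blinks unless zoom is already at that direction's limit.
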(event `self.ReceiveBeginPlay`
  (`SceneComponent.SetVisibility` (`self.PointLight`) false false))

(event `self.Box.OnComponentBeginOverlap`
  (params (OverlappedComponent :type "PrimitiveComponent Object Reference") (OtherActor :type "Actor Object Reference") (OtherComp :type "PrimitiveComponent Object Reference") (OtherBodyIndex :type Integer) (bFromSweep :type Boolean) (SweepResult :type "HitResult Structure (by ref)"))
  (bind _output (`self.GetMinimapArea`))
  (bind _pointlight (`self.PointLight`))
  (bind _zoomvalue (`/Game/FabAsset/ProHUDV2/DemoContent/Blueprints/DemoActor/MinimapMarker/BP_MinimapArea.ZoomValue` (`self.GetMinimapArea`)))
  (bind _zoomvalue_2 (`/Game/FabAsset/ProHUDV2/DemoContent/Blueprints/DemoActor/MinimapMarker/BP_MinimapArea.ZoomValue` (`self.GetMinimapArea`)))
  (cast `/Game/FabAsset/ProHUDV2/DemoContent/DemoCharacter/ThirdPersonCharacter` OtherActor)
  (`|ExecutionSequence`
    (:`then_0`
      (`KismetSystemLibrary.Delay` 0.1)
      (if (`self.ZoomIn`)
        (bind _output_get (set `/Game/FabAsset/ProHUDV2/DemoContent/Blueprints/DemoActor/MinimapMarker/BP_MinimapArea.ZoomValue` (`KismetMathLibrary.FClamp` (+ _zoomvalue_2 0.5) 0.0 2.0) _output))
        (`/Game/FabAsset/ProHUDV2/Blueprints/Libraries/BPi_HUDManagerV2.UpdateMinimap` (`/Game/FabAsset/ProHUDV2/Blueprints/Libraries/BP_PHV2_Functions.GetHUDManager`) _output_get)
        (else
          (bind _output_get_2 (set `/Game/FabAsset/ProHUDV2/DemoContent/Blueprints/DemoActor/MinimapMarker/BP_MinimapArea.ZoomValue` (`KismetMathLibrary.FClamp` (- _zoomvalue_2 0.5) 0.0 2.0) _output))
          (`/Game/FabAsset/ProHUDV2/Blueprints/Libraries/BPi_HUDManagerV2.UpdateMinimap` (`/Game/FabAsset/ProHUDV2/Blueprints/Libraries/BP_PHV2_Functions.GetHUDManager`) _output_get_2))))
    (:`then_1`
      (if (select `bool` (`self.ZoomIn`) :`false` (!= _zoomvalue 0.0) :`true` (!= _zoomvalue 2.0))
        (`SceneComponent.SetVisibility` _pointlight true false)
        (`KismetSystemLibrary.RetriggerableDelay` 0.1)
        (`SceneComponent.SetVisibility` _pointlight false false)
        (`KismetSystemLibrary.RetriggerableDelay` 0.1)
        (`SceneComponent.SetVisibility` _pointlight true false)
        (`KismetSystemLibrary.RetriggerableDelay` 0.5)
        (`SceneComponent.SetVisibility` _pointlight false false)))))

(event `self.Box.OnComponentEndOverlap`
  (params (OverlappedComponent :type "PrimitiveComponent Object Reference") (OtherActor :type "Actor Object Reference") (OtherComp :type "PrimitiveComponent Object Reference") (OtherBodyIndex :type Integer))
  (cast `/Game/FabAsset/ProHUDV2/DemoContent/DemoCharacter/ThirdPersonCharacter` OtherActor))

(fn `GetMinimapArea`
  (returns (Output :type "/Game/FabAsset/ProHUDV2/DemoContent/Blueprints/DemoActor/MinimapMarker/BP_MinimapArea Object Reference"))
  (bind _outactors (`GameplayStatics.GetAllActorsOfClass` "/Game/FabAsset/ProHUDV2/DemoContent/Blueprints/DemoActor/MinimapMarker/BP_MinimapArea.BP_MinimapArea_C"))
  (return (`|GetArrayItem` _outactors)))

(fn `UserConstructionScript`
  (`LightComponent.SetLightColor` (`self.PointLight`) (select `bool` (`self.ZoomIn`) :`false` (struct :`R` 1.0 :`A` 1.0) :`true` (struct :`G` 1.0 :`B` 0.023567 :`A` 1.0) :!type "LinearColor Structure") true))