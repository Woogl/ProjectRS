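; ProHUDV2 demo actor that shows a tutorial notification through the HUD manager when the ThirdPersonCharacter overlaps its box.
; The notification content comes from the TutNotiInfo variable.
; The construction script builds a dynamic material for the billboard, setting its texture, emissive power and a color taken from the notification's highlight color, then applies it as a sized sprite element.
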(event `self.Box.OnComponentBeginOverlap`
  (params (OverlappedComponent :type "PrimitiveComponent Object Reference") (OtherActor :type "Actor Object Reference") (OtherComp :type "PrimitiveComponent Object Reference") (OtherBodyIndex :type Integer) (bFromSweep :type Boolean) (SweepResult :type "HitResult Structure (by ref)"))
  (cast `/Game/FabAsset/ProHUDV2/DemoContent/DemoCharacter/ThirdPersonCharacter` OtherActor)
  (`/Game/FabAsset/ProHUDV2/Blueprints/Libraries/BPi_HUDManagerV2.CreateTutorialNotification` (`/Game/FabAsset/ProHUDV2/Blueprints/Libraries/BP_PHV2_Functions.GetHUDManager`) (`self.TutNotiInfo`)))

(event `UpdateActor`
  (bind _size (`self.Size`))
  (bind (_r _g _b) (break `LinearColor` (`.HighlightColor_8_BD553D1A40A7C2CE09FC099AE01BB0A4` (break `/Game/FabAsset/ProHUDV2/Blueprints/Structs/S_TutNotiInfo` (`self.TutNotiInfo`)))))
  (bind _returnvalue (`KismetMaterialLibrary.CreateDynamicMaterialInstance` (`.Material` (break `MaterialSpriteElement` (`|GetArrayItem` (`MaterialBillboardComponent.Elements` (`self.MaterialBillboard`)))))))
  (set `self.DynamicMaterial` _returnvalue)
  (`MaterialInstanceDynamic.SetTextureParameterValue` (`self.DynamicMaterial`) "Texture" "/Engine/EditorResources/S_Actor.S_Actor")
  (`MaterialInstanceDynamic.SetVectorParameterValue` (`self.DynamicMaterial`) "Color" (`KismetMathLibrary.MakeColor` _r _g _b))
  (`MaterialInstanceDynamic.SetScalarParameterValue` (`self.DynamicMaterial`) "EmissivePower" (`self.EmissivePower`))
  (`MaterialBillboardComponent.SetElements` (`self.MaterialBillboard`) (`|MakeArray` (make `MaterialSpriteElement` :`Material` (`self.DynamicMaterial`) :`BaseSizeX` _size :`BaseSizeY` _size))))

(fn `UserConstructionScript`
  (`self.UpdateActor`))