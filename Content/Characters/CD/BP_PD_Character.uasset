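; BP_PD_Character is a character Blueprint that sets up the game HUD for the locally controlled player once its ability system initializes.
; It pushes WBP_GameHUD onto the UI.Layer.Game layer for player controller 0.
; After the push, it creates and assigns view models for the health, stagger and energy sets, plus two skill abilities looked up by gameplay tag.
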(event `self.PostInitializeAbilitySystem`
  (bind _returnvalue (`AbilitySystemBlueprintLibrary.GetAbilitySystemComponent` null))
  (bind _wbp_game_hud (`self.WBP Game HUD`))
  (if (`self.IsLocallyControlled`)
    (bind (_asynctaskproxy _userwidget) (`AsyncAction_PushContentToLayerForPlayer.PushContentToLayerForPlayer` (`GameplayStatics.GetPlayerController` 0) "/Game/UI/Widgets/WBP_GameHUD.WBP_GameHUD_C" (struct :`TagName` "UI.Layer.Game"))
      (:`AfterPush`
        (set `self.WBP Game HUD` (cast `/Game/UI/Widgets/WBP_GameHUD` _userwidget :!pure true))
        ; Set View Models
        (`|ExecutionSequence`
          (:`then_0`
            (`/Game/UI/Widgets/WBP_GameHUD.SetRsHealthSetViewModel` (`self.WBP Game HUD`) (`RsHealthSetViewModel.CreateHealthSetViewModel` self))
            (`/Game/UI/Widgets/WBP_GameHUD.SetRsStaggerSetViewModel` (`self.WBP Game HUD`) (`RsStaggerSetViewModel.CreateStaggerSetViewModel` self))
            (`/Game/UI/Widgets/WBP_GameHUD.SetRsEnergySetViewModel` (`self.WBP Game HUD`) (`RsEnergySetViewModel.CreateEnergySetViewModel` self)))
          (:`then_1`
            (bind _returnvalue_2 (`RsAbilitySystemLibrary.FindRsAbilityWithTag` _returnvalue (struct :`GameplayTags` (struct :`(TagName` "Ability.Skill.1")))))
            (`/Game/UI/Widgets/WBP_GameHUD.SetRsAbilityViewModel_1` _wbp_game_hud (`RsAbilityViewModel.CreateRsAbilityViewModel` _returnvalue_2)))
          (:`then_2`
            (bind _returnvalue_3 (`RsAbilitySystemLibrary.FindRsAbilityWithTag` _returnvalue (struct :`GameplayTags` (struct :`(TagName` "Ability.Skill.2")))))
            (`/Game/UI/Widgets/WBP_GameHUD.SetRsAbilityViewModel_2` _wbp_game_hud (`RsAbilityViewModel.CreateRsAbilityViewModel` _returnvalue_3))))))))

(fn `UserConstructionScript`)