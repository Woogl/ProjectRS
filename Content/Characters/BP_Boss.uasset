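; BP_Boss is a boss character that registers itself with the game HUD and cleans up when its health runs out.
; On BeginPlay it creates a character view model for itself and passes it to the HUD as the boss view model.
; When the health component reports zero or less, it hides the nameplate, sets a short life span for delayed removal and clears the HUD's boss view model.
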(event `self.ReceiveBeginPlay`
  (bind _returnvalue (`RsUILibrary.GetGameHUD`))
  (bind _returnvalue_2 (`RsCharacterViewModel.CreateRsCharacterViewModel` self))
  (message `/Game/UI/Widgets/Interface/BPI_ViewModelEventProvider.SetBossCharacterViewModel` _returnvalue _returnvalue_2))

(event `self.HealthComponent.OnHealthChange`
  (params (OldValue :type "Float (single-precision)") (NewValue :type "Float (single-precision)") (Instigator :type "Actor Object Reference"))
  (if (<= NewValue 0.0)
    (`SceneComponent.SetHiddenInGame` (`self.NameplateComponent`) true false)
    (`self.SetLifeSpan` 10.0)
    (bind _returnvalue (`RsUILibrary.GetGameHUD`))
    (message `/Game/UI/Widgets/Interface/BPI_ViewModelEventProvider.SetBossCharacterViewModel` _returnvalue null)))

(fn `UserConstructionScript`)