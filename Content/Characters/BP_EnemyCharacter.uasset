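; BP_EnemyCharacter is an enemy character that shows a nameplate and cleans itself up after death.
; On BeginPlay it creates a WBP_Nameplate widget bound to an RsCharacterViewModel built from itself and assigns it to the Nameplate component.
; When HealthComponent reports health at zero or below, it destroys the nameplate and sets a short lifespan so the actor removes itself.
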(event `self.ReceiveBeginPlay`
  (bind _returnvalue (`|CreateWidget` "/Game/UI/Widgets/WBP_Nameplate.WBP_Nameplate_C" null (`RsCharacterViewModel.CreateRsCharacterViewModel` self)))
  (`WidgetComponent.SetWidget` (`self.Nameplate`) _returnvalue))

(event `self.HealthComponent.OnHealthChange`
  (params (OldValue :type "Float (single-precision)") (NewValue :type "Float (single-precision)") (Instigator :type "Actor Object Reference"))
  (if (<= NewValue 0.0)
    (`ActorComponent.K2_DestroyComponent` (`self.Nameplate`))
    (`self.SetLifeSpan` 10.0)))

(fn `UserConstructionScript`)