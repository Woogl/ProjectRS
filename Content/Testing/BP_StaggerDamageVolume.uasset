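; A test volume that repeatedly applies stagger damage, without health damage, to characters standing inside its box.
; On the server, a looping half-second timer gathers every RsCharacterBase overlapping the box.
; Each gets a GE_Damage spec from its own ability system, with set-by-caller health and stagger coefficients, applied with itself as source and target.
; The effect is tagged to trigger a hit reaction.
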(event `self.ReceiveBeginPlay`
  (`/Engine/EditorBlueprintResources/ActorMacros.Switch Has Authority`
    (:`Authority`
      (`KismetSystemLibrary.K2_SetTimerDelegate` (delegate `Apply Effect`) 0.5 true))))

(event `Apply Effect`
  (for _array_element (`PrimitiveComponent.GetOverlappingActors` (`self.Box`) "/Script/Rs.RsCharacterBase")
    (bind _returnvalue (`AbilitySystemBlueprintLibrary.AssignTagSetByCallerMagnitude` (`AbilitySystemComponent.MakeOutgoingSpec` :`self` (`AbilitySystemBlueprintLibrary.GetAbilitySystemComponent` _array_element) :`GameplayEffectClass` "/Game/AbilitySystem/Effects/DamageEffects/GE_Damage.GE_Damage_C") (struct :`TagName` "Coefficient.Damage.Health") 0.0))
    (`AbilitySystemBlueprintLibrary.AssignTagSetByCallerMagnitude` _returnvalue (struct :`TagName` "Coefficient.Damage.Stagger") 0.5)
    (`RsBattleLibrary.ApplyDamageEffectSpec` _array_element _array_element _returnvalue (struct :`GameplayTags` (struct :`(TagName` "Effect.Damage.TriggerHitReaction"))))))

(fn `UserConstructionScript`)